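; Gameplay ability for Pachamama that fires a projectile at the point under a single line trace from the owner.
; On activation it commits, gets instant target data from the trace with debug enabled, and builds a GE_Damage spec with a SetByCaller Data.Damage magnitude.
; It spawns BP_Projectile_Pachamama slightly offset from the avatar on authority only, passing it the trace end point, damage spec and instigator, then ends.
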(event `self.K2_ActivateAbility`
  (`self.K2_CommitAbility`)
  (bind (_asynctaskproxy _data) (`AbilityTask_WaitTargetData.WaitTargetData` "None" "Instant" "/Script/GameplayAbilities.GameplayAbilityTargetActor_SingleLineTrace" 999999.0 (struct :`Name` "NoCollision") true (`self.MakeTargetLocationInfoFromOwnerActor`) (struct) null (struct) true)
    (:`ValidData`
      (bind _returnvalue (`AbilitySystemBlueprintLibrary.AssignTagSetByCallerMagnitude` (`self.MakeOutgoingGameplayEffectSpec` "/Game/GAS/GameplayEffects/GE_Damage.GE_Damage_C") (struct :`TagName` "Data.Damage") -50.0))
      (`GameplayTask_SpawnActor.SpawnActor` null (+ (`Actor.K2_GetActorLocation` (`self.GetAvatarActorFromActorInfo`)) (15.0 0.0 0.0)) (struct) "/Game/Projectile/BP_Projectile_Pachamama.BP_Projectile_Pachamama_C" true 2000.0 (`AbilitySystemBlueprintLibrary.GetTargetDataEndPoint` _data) _returnvalue (cast `Pawn` (`self.GetAvatarActorFromActorInfo`) :!pure true)
        (:`then`
          (`self.K2_EndAbility`))))))