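; GA_Equip_Weapon is an event-triggered gameplay ability that equips or unequips the avatar's weapon.
; It prints the event's first target tag and switches on it, calling the avatar's WeaponManagerComponent to equip the staff weapon for the staff tag or unequip for the default case.
; The ability then ends, but only when that component is valid; without one, EndAbility is never called.
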(event `self.K2_ActivateAbilityFromEvent`
  (params (EventData :type "GameplayEventData Structure (by ref)"))
  (bind _returnvalue (`Actor.GetComponentByClass` (`self.GetAvatarActorFromActorInfo`) "/Script/AmaruShooter.WeaponManagerComponent"))
  (bind _output (`|GetArrayItem` (`BlueprintGameplayTagLibrary.BreakGameplayTagContainer` (`.TargetTags` (break `GameplayEventData` EventData)))))
  (`KismetSystemLibrary.PrintString` (`BlueprintGameplayTagLibrary.GetDebugStringFromGameplayTag` _output))
  (`/Engine/EditorBlueprintResources/StandardMacros.IsValid` _returnvalue
    (:`Is Valid`
      (`|ExecutionSequence`
        (:`then_0`
          (`|SwitchGameplayTag` _output
            (:`Default`
              (`WeaponManagerComponent.UnequipWeapon` _returnvalue))
            (:`Weapon.Range.Staff`
              (`WeaponManagerComponent.EquipWeapon` _returnvalue "/Game/Weapons/BP_StaffWeapon.BP_StaffWeapon_C"))))
        (:`then_1`
          (`self.K2_EndAbility`))))))