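; Gameplay ability for Wayra's shot, which spawns a projectile-style actor from the first-person character's muzzle toward its aim point.
; On activation it builds a GE_Damage spec with a set-by-caller Data.Damage magnitude.
; The authority-only spawn receives the spec, speed, target location and instigator, leaving damage application to the spawned actor, and the ability then ends.
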(event `self.K2_ActivateAbility`
  (bind _asbp_first_person_character (cast `/Game/FirstPerson/Blueprints/BP_FirstPersonCharacter` (`self.GetAvatarActorFromActorInfo`)))
  (bind _spawbulletsocket (`/Game/FirstPerson/Blueprints/BP_FirstPersonCharacter.GetMuzzleSpawnPoint` _asbp_first_person_character))
  (bind _aimpoint (`/Game/FirstPerson/Blueprints/BP_FirstPersonCharacter.GetAimPoint` _asbp_first_person_character))
  (bind _returnvalue (`AbilitySystemBlueprintLibrary.AssignTagSetByCallerMagnitude` (`self.MakeOutgoingGameplayEffectSpec` "/Game/GAS/GameplayEffects/GE_Damage.GE_Damage_C") (struct :`TagName` "Data.Damage") -20.0))
  (`GameplayTask_SpawnActor.SpawnActor` null _spawbulletsocket (`KismetMathLibrary.FindLookAtRotation` _spawbulletsocket _aimpoint) "/Game/Projectile/BP_Projectile_Wayra.BP_Projectile_Wayra_C" true 500.0 _aimpoint _returnvalue (cast `Pawn` (`self.GetAvatarActorFromActorInfo`) :!pure true)
    (:`then`
      (`self.K2_EndAbility`))))