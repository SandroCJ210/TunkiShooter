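; Gameplay ability that gives Wayra a short, fast dash.
; On activation it commits, then applies a constant root motion force along the last movement input, or actor forward when there is no input.
; A dash gameplay cue plays while the ability is active and is removed when it ends.
; The ability ends when the force finishes, clamping exit velocity to the pawn's max movement speed, with a fallback for non-pawn avatars.
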(event `self.K2_ActivateAbility`
  (`self.K2_CommitAbility`)
  (`AbilityTask_ApplyRootMotionConstantForce.ApplyRootMotionConstantForce` "None" (`self.GetDashDirection`) 2000.0 0.2 false null "ClampVelocity" (0.0 0.0 0.0) (`self.GetMaxSpeed`)
    (:`then`
      (`self.K2_AddGameplayCue` (struct :`TagName` "GameplayCue.Dash.Active")))
    (:`OnFinish`
      (`self.K2_EndAbility`))))

(fn `GetDashDirection`
  (returns (OutDirection :type "Vector Structure"))
  (bind _returnvalue (`self.GetAvatarActorFromActorInfo`))
  (bind _aspawn (cast `Pawn` _returnvalue))
  (bind _returnvalue_2 (`Pawn.GetLastMovementInputVector` _aspawn))
  (if (`KismetMathLibrary.Vector_IsZero` _returnvalue_2)
    (return (`Actor.GetActorForwardVector` _returnvalue))
    (else
      (return _returnvalue_2))))

(fn `GetMaxSpeed`
  (returns (`Max Speed` :type "Float (double-precision)"))
  (bind _aspawn (cast `Pawn` (`self.GetAvatarActorFromActorInfo`))
    (:`then`
      (return (`MovementComponent.GetMaxSpeed` (`Pawn.GetMovementComponent` _aspawn))))
    (:`CastFailed`
      (return 600.0))))